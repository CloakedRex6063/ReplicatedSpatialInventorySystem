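; BP_PC is a player controller that connects the player's input to an inventory component and its UI.
; On BeginPlay, the local controller initializes the component with the controlled BP_BaseCharacter and creates an inventory widget bound to it.
; Input actions trigger pickup on the component or toggle the widget, switching input mode and cursor visibility.
; GetLocationToDrop returns a point just in front of the controlled pawn.
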(event EventBeginPlay
  (bind _inventorycomponent (Variables|Default|GetInventoryComponent))
  ;[0 0 0] Create Inventory Widget
  (if (Pawn|IsLocalController)
    (Default|Initialize _inventorycomponent (.AsBP%20Base%20Character (Utilities|Casting|CastToBP_BaseCharacter (Pawn|GetControlledPawn))))
    (bind _returnvalue (UserInterface|CreateWidget "/Game/UI/Inventory/UI_Inventory.UI_Inventory_C" self _inventorycomponent 5e+01))
    (Variables|Default|SetInventory _returnvalue)))

(event Input|ActionEvents|InputActionPickup/Interact
  (params (Key :type Key%20Structure :default "None"))
  ;[0 0 0] Pickup Item
  (:Pressed
    (Default|Pickup (Variables|Default|GetInventoryComponent))))

(event Input|ActionEvents|InputActionInventory
  (params (Key :type Key%20Structure :default "None"))
  (bind _self self)
  (bind _inventory (Variables|Default|GetInventory))
  ;[0 0 0] Toggle Inventory
  (:Pressed
    (if (Variables|Default|GetInventoryOpen?)
      (Widget|RemovefromParent _inventory)
      (Variables|Default|SetInventoryOpen? false)
      (Input|SetInputModeGameOnly _self)
      (Variables|Default|SetbShowMouseCursor false)
      (else
        (UserInterface|Viewport|AddtoViewport _inventory 0)
        (Variables|Default|SetInventoryOpen? true)
        (Input|SetInputModeGameandUI _self (Variables|Default|GetInventory) "DoNotLock" false)
        (Variables|Default|SetbShowMouseCursor true)))))

(fn ConstructionScript)

(fn GetLocationtoDrop
  (bind _returnvalue (Pawn|GetControlledPawn))
  (return (+ (Transformation|GetActorLocation _returnvalue) (* (Transformation|GetActorForwardVector _returnvalue) 5e+01))))