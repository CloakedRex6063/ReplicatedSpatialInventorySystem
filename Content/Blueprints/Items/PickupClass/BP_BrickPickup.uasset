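; BP_BrickPickup is a brick item pickup that defines how the brick is represented as an item object.
; Its GetDefaultItemObject function constructs a BP_Object with a two-by-one footprint, normal and rotated brick icons, and its own class as the item class.
; The event graph holds only disabled placeholder events, and the construction script just calls the parent.
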(event EventBeginPlay
  (|CallParentFunction) ; This node is disabled and will not be called.\nDrag off pins to build functionality.
)

(event Collision|EventActorBeginOverlap
  (params (OtherActor :type Actor%20Object%20Reference))
  (|CallParentFunction OtherActor) ; This node is disabled and will not be called.\nDrag off pins to build functionality.
)

(event EventTick
  (params (DeltaSeconds :type Float%20%28single-precision%29))
  (|CallParentFunction DeltaSeconds) ; This node is disabled and will not be called.\nDrag off pins to build functionality.
)

(fn ConstructionScript
  (|CallParentFunction))

(fn GetDefaultItemObject
  (bind _returnvalue (Game|ConstructObjectfromClass "/Game/Blueprints/Items/Actual_Items/BP_Object.BP_Object_C" self (Utilities|Struct|MakeIntPoint 2 1) "/Game/Materials/Item/M_Brick.M_Brick" "/Game/Materials/Item/M_Brick_Rotated.M_Brick_Rotated" "BP_BrickPickup_C"))
  (return _returnvalue))