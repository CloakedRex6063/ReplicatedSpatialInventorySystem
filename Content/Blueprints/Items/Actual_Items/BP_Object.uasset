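; BP_Object is an item data object that describes an item's footprint, icon and class, with support for rotation.
; Rotate toggles the Rotated flag, which makes GetDimensions swap X and Y and GetIcon return RotatedIcon instead of Icon.
; Simple getters expose the rotation state and the stored ItemClass.
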(fn GetDimensions
  (bind _dimensions (Variables|Default|GetDimensions))
  (return (select (Variables|Default|GetRotated) (Utilities|Struct|MakeIntPoint (.y _dimensions) (.x _dimensions)) (Variables|Default|GetDimensions))))

(fn GetIcon
  (return (select (Variables|Default|GetRotated) (Variables|Default|GetRotatedIcon) (Variables|Default|GetIcon))))

(fn GetItemClass
  (return (Variables|Default|GetItemClass)))

(fn Rotate
  (Variables|Default|SetRotated (not (Variables|Default|GetRotated))))

(fn IsRotated?
  (return (Variables|Default|GetRotated)))