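; Inventory component that gives a character a grid inventory of multi-tile items, with world pickup and dropping.
; A looping timer sphere-traces from the camera to find and outline BP_BaseItemPickup actors via custom depth.
; Pickup scans a flattened tile array for room, retrying once rotated, fills every covered slot, then destroys the actor through a server event.
; A dirty flag defers change notifications to Tick, and another server event spawns items in front of the character.
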(event Custom|Initialize
  (params (Character :type BP%20Base%20Character%20Object%20Reference))
  (Utilities|IsValid Character
    (:Is%20Valid
      (Variables|Default|SetCharacter Character))))

(event EventTick
  (params (DeltaSeconds :type Float%20%28single-precision%29))
  (if (Variables|Default|GetIsDirty?)
    (Variables|Default|SetIsDirty? false)
    (Default|CallOnInventoryChanged)))

(event EventBeginPlay
  (Utilities|Time|SetTimerbyFunctionName 0 "LineTraceForItemCheck" 0.01 true)
  (Utilities|Array|Resize (Variables|Default|GetInventoryItems) (* (Variables|Constants|GetColumns) (Variables|Constants|GetRows))))

(event Custom|Server_DestroyItem
  (params (Actor :type Actor%20Object%20Reference))
  ;[0 0 0] Destroy Item on Server
  (Actor|DestroyActor Actor))

(event Custom|Server_SpawnItem
  (params (ItemObject :type BP%20Base%20Item%20Pickup%20Class%20Reference))
  ;[0 0 0] Spawn item on Server
  (CallFunction|SpawnItemfromActor ItemObject))

(fn TrytoAddItem
  (params (Object :type BP%20Object%20Object%20Reference))
  (Utilities|IsValid Object
    (:Is%20Valid
      (for (_ _array_index) (Variables|Default|GetInventoryItems) :!label _label
        (bind _return (CallFunction|IsRoomAvailable Object _array_index))
        (if _return
          (CallFunction|AddItemat Object _array_index)
          (return true)))
      (Utilities|FlowControl|Sequence
        (:then_0
          (Utilities|FlowControl|DoOnce false
            (:Completed
              (Default|Rotate Object)
              (goto _label))))
        (:then_1
          (Default|Rotate Object)
          (return false))))))

(fn LineTraceforItemCheck
  (bind _character (Variables|Default|GetCharacter))
  (bind _camera (Variables|/Game/Blueprints/Character/BP_BaseCharacter.BP_BaseCharacter_C|GetCamera _character))
  (bind _returnvalue (Transformation|GetWorldLocation _camera))
  (Utilities|IsValid _character
    (:Is%20Valid
      (bind (_outhit _returnvalue_2) (Collision|SphereTraceByChannel _returnvalue (+ _returnvalue (* (Math|Vector|GetForwardVector _camera) (Variables|Default|GetMaxPickupDistance))) 1e+01 "TraceTypeQuery1" false 0 "None"))
      (if _returnvalue_2
        (bind _asbp_base_item_pickup (Utilities|Casting|CastToBP_BaseItemPickup (.HitActor (Collision|BreakHitResult _outhit)))
          (:then
            (bind _output_get (Variables|Default|SetItem _asbp_base_item_pickup))
            (Rendering|SetRenderCustomDepth (Variables|/Game/Blueprints/Items/PickupClass/BP_BaseItemPickup.BP_BaseItemPickup_C|GetStaticMesh _output_get) true))
          (:CastFailed
            (Utilities|IsValid (Variables|Default|GetItem) :!label _label
              (:Is%20Valid
                (Rendering|SetRenderCustomDepth (Variables|/Game/Blueprints/Items/PickupClass/BP_BaseItemPickup.BP_BaseItemPickup_C|GetStaticMesh (Variables|Default|GetItem)) false)
                (Variables|Default|SetItem 0)))))
        (else
          (goto _label))))))

(fn Pickup
  (bind _item (Variables|Default|GetItem))
  (Utilities|IsValid _item
    (:Is%20Valid
      (bind _added (CallFunction|TrytoAddItem (Variables|/Game/Blueprints/Items/PickupClass/BP_BaseItemPickup.BP_BaseItemPickup_C|GetItemObject _item)))
      (if _added
        (CallFunction|ServerDestroyItem _item)))))

(fn IsRoomAvailable
  (params (ItemObject :type BP%20Object%20Object%20Reference) (TopLeftIndex :type Integer))
  (Utilities|FlowControl|Sequence
    (:then_0
      (bind _tile (Utilities|ForEachIndex ItemObject TopLeftIndex)
        (:LoopBody
          (Utilities|IsTileValid _tile
            (:true
              (bind (_item _returnvalue) (CallFunction|GetItematIndex (CallFunction|TiletoIndex _tile)))
              (if _returnvalue
                (Utilities|IsValid _item
                  (:Is%20Valid
                    (return false)))
                (else
                  (return false))))
            (:false
              (return false))))))
    (:then_1
      (return true))))

(fn IndextoTile
  (params (Index :type Integer))
  (bind _columns (Variables|Constants|GetColumns))
  (return (Utilities|Struct|MakeTiles (Math|Integer|%(Integer) Index _columns) (/ Index _columns))))

(fn GetItematIndex
  (params (IndexToTest :type Integer))
  (if (Utilities|Array|IsValidIndex (Variables|Default|GetInventoryItems) IndexToTest)
    (return (Utilities|Array|Get(acopy) (Variables|Default|GetInventoryItems) IndexToTest) true)
    (else
      (return 0 false))))

(fn TiletoIndex
  (params (Tile :type Tiles%20Structure))
  (bind (_x _y) (Utilities|Struct|BreakTiles Tile))
  (return (+ _x (* _y (Variables|Constants|GetColumns)))))

(fn AddItemat
  (params (ItemObject :type BP%20Object%20Object%20Reference) (TopLeftIndex :type Integer))
  (bind _tile (Utilities|ForEachIndex ItemObject TopLeftIndex)
    (:LoopBody
      (Utilities|Array|SetArrayElem (Variables|Default|GetInventoryItems) (CallFunction|TiletoIndex _tile) ItemObject))
    (:Completed
      (Variables|Default|SetIsDirty? true))))

(fn GetAllItems
  (for (_array_element _array_index) (Variables|Default|GetInventoryItems)
    (bind _output_get (LocalVariables|SetCurrentItem%28Local%29 _array_element))
    (Utilities|IsValid _output_get
      (:Is%20Valid
        (if (not (Utilities|Map|Contains (LocalVariables|GetAllItems%28Local%29) _array_element))
          (Utilities|Map|Add (LocalVariables|GetAllItems%28Local%29) (LocalVariables|GetCurrentItem%28Local%29) (CallFunction|IndextoTile _array_index))))))
  (return (LocalVariables|GetAllItems%28Local%29)))

(fn RemoveItem
  (params (ItemObject :type BP%20Object%20Object%20Reference))
  (Utilities|IsValid ItemObject
    (:Is%20Valid
      (for (_array_element _array_index) (Variables|Default|GetInventoryItems)
        (if (== _array_element ItemObject)
          (Utilities|Array|SetArrayElem (Variables|Default|GetInventoryItems) _array_index 0)
          (Variables|Default|SetIsDirty? true))))))

(fn SpawnItemfromActor
  (params (ItemClass :type BP%20Base%20Item%20Pickup%20Class%20Reference))
  (bind _character (Variables|Default|GetCharacter))
  (Utilities|FlowControl|Sequence
    (:then_0
      (LocalVariables|SetSpawnLocation (+ (Transformation|GetActorLocation _character) (* (Transformation|GetActorForwardVector _character) 1.5e+02))))
    (:then_1
      (Game|SpawnActorfromClass ItemClass (Math|Transform|MakeTransform (LocalVariables|GetSpawnLocation) "0, 0, 0" "1,1,1") "Undefined" 0 0))))